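; BP_MyCharacter is a character Blueprint that connects its singing component to an on-screen note UI.
; On BeginPlay it builds a UMG_Box widget with columns from the component's note count and bar offset, then hides it.
; Component delegates move the bar, set the current note column's image opacity and toggle visibility.
; When singing starts, a short delay precedes feeding the widget's measured sizes back to the component, guarded by IsCall.
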(event Custom|OnStartSinging
  (params (StartSinging :type Boolean))
  ;[1 1 1] Display UI or hide on singing
  (if StartSinging
    (Widget|SetVisibility (Variables|Default|GetUMG_Box) "Visible")
    (if (not (Variables|Default|GetIsCall))
      (Utilities|FlowControl|Delay 0.1)
      ;;[1 -2.208 -34.2 9.475 20] UI IS NUL À CHIER, JSP KOMENT AVOIR LA TAILLE
      (bind (_size _imagesize) (Default|GetSize (Variables|Default|GetUMG_Box)))
      (Class|SingingComponent|SetUIImageSize (Variables|Default|GetSingingComponent) _imagesize)
      (Class|SingingComponent|SetUISize (Variables|Default|GetSingingComponent) _size)
      (Development|PrintString (Utilities|String|ToString(Float) _size)))
    (else
      (Widget|SetVisibility (Variables|Default|GetUMG_Box) "Collapsed"))))

(event Custom|Sing
  (params (SingNote :type ESingButton%20Enum :default "Earth"))
  ;[1 1 1] Show input in UI on start Singing
  (bind _newparam (Default|GetVerticalBox (Variables|Default|GetUMG_Box) (Class|SingingComponent|GetCurrentNote (Variables|Default|GetSingingComponent))))
  (Default|SetImageOpacity _newparam SingNote))

(event Custom|OnSingingHold
  (params (Position :type Float%20%28single-precision%29))
  (Default|SetBarPosition (Variables|Default|GetUMG_Box) Position))

(event EventBeginPlay
  (EventDispatchers|AssignOnEchoSingingBarPercent (Variables|Default|GetSingingComponent) (delegate Custom|OnSingingHold))
  (EventDispatchers|BindEventtoOnSingingDelegate (Variables|Default|GetSingingComponent) (delegate Custom|Sing))
  ;[1 1 1] Display UI or hide on singing
  (EventDispatchers|BindEventtoStartSingingDelegate (Variables|Default|GetSingingComponent) (delegate Custom|OnStartSinging))
  ;[1 1 1] Setup UI
  (bind _returnvalue (UserInterface|CreateWidget "/Game/UI/UMG_Box.UMG_Box_C" (Game|GetPlayerController 0)))
  (bind _output_get (Variables|Default|SetUMG_Box _returnvalue))
  (Variables|/Game/UI/UMG_Box.UMG_Box_C|SetColumnsCount _output_get (Class|SingingComponent|GetNumberOfNotes (Variables|Default|GetSingingComponent)))
  (Variables|/Game/UI/UMG_Box.UMG_Box_C|SetBarOffset _output_get (Class|SingingComponent|GetBarOffset (Variables|Default|GetSingingComponent)))
  (Default|GenerateColumns _output_get)
  (UserInterface|Viewport|AddtoViewport _output_get 0)
  (Widget|SetVisibility _output_get "Collapsed"))

(fn ConstructionScript)