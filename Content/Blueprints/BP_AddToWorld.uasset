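; BP_AddToWorld is an actor that presents a UMG_Box widget through its Widget component.
; On BeginPlay it copies its ColumnCount into the widget and has it generate its columns.
; A GetUMGBox helper returns the cast widget to callers.
; A two-second eased view blend to the owner of Camera is present but unconnected, so it never runs.
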(event EventBeginPlay
  (bind _asumg_box (Utilities|Casting|CastToUMG_Box (UserInterface|GetUserWidgetObject (Variables|Default|GetWidget))))
  (Variables|/Game/UI/UMG_Box.UMG_Box_C|SetColumnsCount _asumg_box (Variables|Default|GetColumnCount))
  (Default|GenerateColumns _asumg_box))

(fn ConstructionScript)

(fn GetUMGBox
  (bind _asumg_box (Utilities|Casting|CastToUMG_Box (UserInterface|GetUserWidgetObject (Variables|Default|GetWidget))))
  (return _asumg_box))